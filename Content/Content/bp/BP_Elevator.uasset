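; Elevator actor that carries the player, freezing their movement while it rises.
; BeginPlay caches the third-person character; overlapping the Stop component disables its movement, then a DoOnce activates InterpToMovement and restores control after a short delay.
; Later overlaps still freeze the player but never reach the release.
; A separate CrashBandcout event plays the High timeline into SetActorLocation, with its scaled height output left unconnected.
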(event OnComponentBeginOverlap(Stop)
  (params (OverlappedComponent :type Primitive%20Component%20Object%20Reference) (OtherActor :type Actor%20Object%20Reference) (OtherComp :type Primitive%20Component%20Object%20Reference) (OtherBodyIndex :type Integer) (bFromSweep :type Boolean) (SweepResult :type Hit%20Result%20Structure%20%28by%20ref%29))
  ;[0.15 0.15 0.15 0.5] Lorsque le joueur est dans l'ascenseur, le stop pendant 1.1s soit le temps que l'ascenseur mais pour monter
  (if (== OtherActor (Variables|Default|GetAs%20BP%20Third%20Person%20Character))
    (Default|Don'tMove (Variables|Default|GetAs%20BP%20Third%20Person%20Character))
    (Utilities|FlowControl|DoOnce false
      (:Completed
        (Components|Activation|Activate (Variables|Default|GetInterpToMovement) false)
        (Utilities|FlowControl|Delay 1.1)
        (Default|MoveAgain (Variables|Default|GetAs%20BP%20Third%20Person%20Character))))))

(event Custom|CrashBandcout
  ;[0.15 0.15 0.15 0.5] CustomEvent qui augmente la hauteur (position) de l'acteur
  (bind _float (Timeline|High Play)
    (:Update
      (Transformation|SetActorLocation self (Math|Vector|MakeVector 0.0 0.0 0.0) false false))))

(event EventBeginPlay
  ;[0.15 0.15 0.15 0.5] Setup du as BP_TPS
  (bind _asbp_third_person_character (Utilities|Casting|CastToBP_ThirdPersonCharacter (Game|GetPlayerCharacter 0)))
  (Variables|Default|SetAs%20BP%20Third%20Person%20Character _asbp_third_person_character))

(fn ConstructionScript)