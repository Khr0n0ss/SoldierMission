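; BP_Light is a light Blueprint whose PointLight flickers continuously during play.
; The construction script applies the base Intensity to the light.
; From BeginPlay, a self-looping Retriggerable Delay waits a random time between MinTime and MaxTime, then a FlipFlop alternates the light between MinFlickerIntensity and Intensity.
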(event EventBeginPlay
  (bind _pointlight (Variables|Default|GetPointLight))
  ;[0.15 0.15 0.15 0.5] Flickering de la light
  (Utilities|FlowControl|RetriggerableDelay (Math|Random|RandomFloatinRange (Variables|Default|GetMinTime) (Variables|Default|GetMaxTime)) :!label _label)
  (Utilities|FlowControl|FlipFlop
    (:A
      (Rendering|Components|Light|SetIntensity _pointlight (Variables|Default|GetMinFlickerIntensity))
      (goto _label))
    (:B
      (Rendering|Components|Light|SetIntensity _pointlight (Variables|Default|GetIntensity))
      (goto _label))))

(fn ConstructionScript
  ;[0.15 0.15 0.15 0.5] Set l'intensité de la lumière
  (Rendering|Components|Light|SetIntensity (Variables|Default|GetPointLight) (Variables|Default|GetIntensity)))