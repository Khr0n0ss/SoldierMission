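; BP_IA is an AI enemy that damages what it spots and can be killed.
; Each PawnSensing sighting fires a debug-drawn 500-unit line trace along GetOwner's forward vector, not toward the seen pawn, applying damage to the hit actor.
; Incoming damage lowers HP stored in the BP_IA_huda widget itself, destroying the actor at zero or below.
; SphereBox overlaps show and hide that health bar.
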(event OnSeePawn(PawnSensing)
  (params (Pawn :type Pawn%20Object%20Reference))
  ;[0.15 0.15 0.15 0.5] Tant que le joueur est dans le champs de vision, il prend des dégats en continue cool nan ?
  (CallFunction|LineTrace))

(event OnComponentBeginOverlap(SphereBox)
  (params (OverlappedComponent :type Primitive%20Component%20Object%20Reference) (OtherActor :type Actor%20Object%20Reference) (OtherComp :type Primitive%20Component%20Object%20Reference) (OtherBodyIndex :type Integer) (bFromSweep :type Boolean) (SweepResult :type Hit%20Result%20Structure%20%28by%20ref%29))
  ;[0.15 0.15 0.15 0.5] Barre d'HP visible
  (Rendering|SetVisibility (Variables|Default|GetHealthBarWidget) true false))

(event OnComponentEndOverlap(SphereBox)
  (params (OverlappedComponent :type Primitive%20Component%20Object%20Reference) (OtherActor :type Actor%20Object%20Reference) (OtherComp :type Primitive%20Component%20Object%20Reference) (OtherBodyIndex :type Integer))
  ;[0.15 0.15 0.15 0.5] Barre d'HP invisible
  (Rendering|SetVisibility (Variables|Default|GetHealthBarWidget) false false))

(event Game|Damage|EventAnyDamage
  (params (Damage :type Float%20%28single-precision%29) (DamageType :type Damage%20Type%20Object%20Reference) (InstigatedBy :type Controller%20Object%20Reference) (DamageCauser :type Actor%20Object%20Reference))
  ;[0.15 0.15 0.15 0.5] Si IA prend des damages alors pv diminué et actualisé sur le widget et si pv <= à 0 alors mort
  (Variables|Default|SetDamage Damage)
  (bind _asbp_ia_huda (Utilities|Casting|CastToBP_IA_huda (UserInterface|GetUserWidgetObject (Variables|Default|GetHealthBarWidget))))
  (bind _output_get (Variables|Default|SetAs%20BP%20IA%20Huda _asbp_ia_huda))
  (bind _output_get_2 (Variables|/Game/Content/hud/BP_IA_huda.BP_IA_huda_C|SetHP _output_get (- (Variables|/Game/Content/hud/BP_IA_huda.BP_IA_huda_C|GetHP (Variables|Default|GetAs%20BP%20IA%20Huda)) (Variables|Default|GetDamage))))
  (if (<= _output_get_2 0.0)
    (Actor|DestroyActor self)))

(fn ConstructionScript)

(fn LineTrace
  (bind _returnvalue (Components|GetOwner))
  (bind _returnvalue_2 (Transformation|GetActorLocation _returnvalue))
  ;[0.15 0.15 0.15 0.5] LineTrace de damage
  (bind _outhit (Collision|LineTraceByChannel _returnvalue_2 (+ _returnvalue_2 (* (Transformation|GetActorForwardVector _returnvalue) 5e+02)) "TraceTypeQuery3" false 0 "ForDuration" true "(R=1.000000,G=0.000000,B=0.000000,A=1.000000)" "(R=0.000000,G=1.000000,B=0.000000,A=1.000000)" 1.0))
  (Game|Damage|ApplyDamage (.HitActor (Collision|BreakHitResult _outhit)) 2.0 0 0))